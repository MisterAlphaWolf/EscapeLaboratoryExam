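; BP_BrokenDoor is a sliding double lab door that opens when something overlaps its Collision component and closes when the overlap ends.
; Both overlap events set open/close flags and start a fast looping timer, which appears to drive MoveDoor.
; MoveDoor steps the two panels in opposite directions along local Y, clearing the timer at either limit.
; Closing requires DoorOpen, so leaving before full opening stalls the panels part-open.
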(event `self.Collision.OnComponentBeginOverlap`
  (params (OverlappedComponent :type "PrimitiveComponent Object Reference") (OtherActor :type "Actor Object Reference") (OtherComp :type "PrimitiveComponent Object Reference") (OtherBodyIndex :type Integer) (bFromSweep :type Boolean) (SweepResult :type "HitResult Structure (by ref)"))
  ;[0 0.3281 0] SecurityBreach0X00CF52
  (set `self.CloseDoor` false)
  (set `self.OpenDoor` true)
  (bind _returnvalue (`KismetSystemLibrary.K2_SetTimerDelegate` (`|CreateDelegate` :!event `MoveDoor`) 0.015 true :!label _label))
  (set `self.MoveDoorTimerHandle` _returnvalue))

(event `self.Collision.OnComponentEndOverlap`
  (params (OverlappedComponent :type "PrimitiveComponent Object Reference") (OtherActor :type "Actor Object Reference") (OtherComp :type "PrimitiveComponent Object Reference") (OtherBodyIndex :type Integer))
  ;[0 0.3281 0] SecurityBreach0X00CF52
  (set `self.OpenDoor` false)
  (set `self.CloseDoor` true)
  (goto _label))

(event `MoveDoor`
  (bind _doorposition (`self.DoorPosition`))
  (bind _doorposition_2 (`self.DoorPosition`))
  ;[0 0.3281 0] SecurityBreach0X00CF52
  (if (`self.OpenDoor`)
    (`/Engine/EditorBlueprintResources/StandardMacros.CompareFloat` _doorposition_2 90.0
      (:`>`
        (set `self.DoorPosition` 90.0 :!label _label_2)
        (set `self.DoorOpen?` true)
        (`KismetSystemLibrary.K2_ClearAndInvalidateTimerHandle` (`self.MoveDoorTimerHandle`)))
      (:`==`
        (goto _label_2))
      (:`<`
        (set `self.DoorPosition` (+ _doorposition_2 4.0))
        (`SceneComponent.K2_SetRelativeLocation` (`self.LabDoor03B`) (`KismetMathLibrary.MakeVector` 0.0 (`self.DoorPosition`)) false false)
        (`SceneComponent.K2_SetRelativeLocation` (`self.LabDoor03A`) (`KismetMathLibrary.MakeVector` 0.0 (* (`self.DoorPosition`) -1.0)) false false)))
    (elif (and (`self.DoorOpen?`) (`self.CloseDoor`))
      (`/Engine/EditorBlueprintResources/StandardMacros.CompareFloat` _doorposition
        (:`>`
          (set `self.DoorPosition` (- _doorposition 4.0))
          (`SceneComponent.K2_SetRelativeLocation` (`self.LabDoor03B`) (`KismetMathLibrary.MakeVector` 0.0 (`self.DoorPosition`)) false false)
          (`SceneComponent.K2_SetRelativeLocation` (`self.LabDoor03A`) (`KismetMathLibrary.MakeVector` 0.0 (* (`self.DoorPosition`) -1.0)) false false))
        (:`==`
          (set `self.DoorPosition` 0.0 :!label _label_3)
          (set `self.CloseDoor` true)
          (set `self.DoorOpen?` false)
          (`KismetSystemLibrary.K2_ClearAndInvalidateTimerHandle` (`self.MoveDoorTimerHandle`)))
        (:`<`
          (goto _label_3))))))

(fn `UserConstructionScript`)